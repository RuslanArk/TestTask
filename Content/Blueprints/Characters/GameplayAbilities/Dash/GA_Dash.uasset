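; Gameplay ability for a dash attack that launches the character forward through other pawns, damaging, knocking back and stunning those it hits.
; Activation zeroes ground friction, sets pawn collision to overlap, applies a velocity-change impulse and plays the dash montage.
; Deal-damage gameplay events apply the damage effect and push the target away from the dasher.
; Montage completion, blend-out, interruption or cancellation restores friction and blocking collision, then ends the ability.
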(event Ability|EventActivateAbility
  (Ability|CommitAbility)
  (bind _ascharacter (Utilities|Casting|CastToCharacter (Ability|GetOwningActorfromActorInfo))
    (:then
      (Variables|Default|SetOriginal%20Ground%20Friction (Variables|/Script/Engine.CharacterMovementComponent|GetGroundFriction (Variables|/Script/Engine.Character|GetCharacterMovement _ascharacter)))
      (Variables|/Script/Engine.CharacterMovementComponent|SetGroundFriction (Variables|/Script/Engine.Character|GetCharacterMovement _ascharacter) 0.0)
      (bind _basecharacter (CallFunction|GetPlayerCharacterandController))
      (Default|SetCollisiontoPawn _basecharacter "ECR_Overlap")
      (Physics|AddImpulse (Variables|/Script/Engine.Character|GetCharacterMovement _ascharacter) (* (Transformation|GetActorForwardVector _ascharacter) 2e+03) true)
      (|PlayMontageandWaitProxy "None" "/Game/Blueprints/Characters/Animation/AM_Shinbi_Dash.AM_Shinbi_Dash" 1.0 "None" true 1.0 0.0
        (:then
          (bind _payload (Ability|Tasks|WaitGameplayEvent "(TagName=\"skill.dash.dealDamage\")" 0)
            (:EventReceived
              (GameplayEffects|ApplyGameplayEffectToTarget (Ability|TargetData|AbilityTargetDatafromActor (.Target (Utilities|Struct|BreakGameplayEventData _payload))) "/Game/Blueprints/Characters/GameplayAbilities/Dash/GE_Dash_DealDamage.GE_Dash_DealDamage_C" 1 1)
              (bind _asbp_base_character (Utilities|Casting|CastToBP_BaseCharacter (.Target (Utilities|Struct|BreakGameplayEventData _payload))))
              (Default|PushCharacter _asbp_base_character (Math|Vector|Normalize (- (Transformation|GetActorLocation (.Target (Utilities|Struct|BreakGameplayEventData _payload))) (Transformation|GetActorLocation (Ability|GetOwningActorfromActorInfo)))) 4e+03 5.0))))
        (:OnCompleted
          (Variables|/Script/Engine.CharacterMovementComponent|SetGroundFriction (Variables|/Script/Engine.Character|GetCharacterMovement _ascharacter) (Variables|Default|GetOriginal%20Ground%20Friction) :!label _label)
          (bind _basecharacter_2 (CallFunction|GetPlayerCharacterandController))
          (Default|SetCollisiontoPawn _basecharacter_2 "ECR_Block")
          (Ability|EndAbility))
        (:OnBlendOut
          (goto _label))
        (:OnInterrupted
          (goto _label))
        (:OnCancelled
          (goto _label))))
    (:CastFailed
      (Ability|EndAbility))))

(event Ability|EventOnEndAbility
  (params (bWasCancelled :type Boolean)))