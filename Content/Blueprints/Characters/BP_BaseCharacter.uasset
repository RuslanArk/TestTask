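; BP_BaseCharacter is a combat character base that uses the Gameplay Ability System for melee, dash and health regen.
; It acquires the three abilities on BeginPlay and activates each by class through its own event.
; Sword and capsule overlaps send damage gameplay events to itself targeting hostile characters, with an exclusion list preventing repeat dash hits.
; It also handles montage-timed death, capsule Pawn collision switching, and knockback with temporarily zero friction and optional stun.
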(event OnComponentBeginOverlap(CapsuleComponent)
  (params (OverlappedComponent :type Primitive%20Component%20Object%20Reference) (OtherActor :type Actor%20Object%20Reference) (OtherComp :type Primitive%20Component%20Object%20Reference) (OtherBodyIndex :type Integer) (bFromSweep :type Boolean) (SweepResult :type Hit%20Result%20Structure%20%28by%20ref%29))
  (bind _self self)
  (bind _overlappedexclude (Variables|Default|GetOverlappedExclude))
  (bind _asbp_base_character (Utilities|Casting|CastToBP_BaseCharacter OtherActor))
  (bind _returnvalue (Class|BaseCharacter|IsHostile _asbp_base_character _self))
  (if _returnvalue
    (if (not (Utilities|Array|ContainsItem _overlappedexclude _asbp_base_character))
      (Utilities|Array|AddUnique _overlappedexclude _asbp_base_character)
      (Ability|SendGameplayEventtoActor self "(TagName=\"skill.dash.dealDamage\")" (Utilities|Struct|MakeGameplayEventData "(TagName=\"\")" _self OtherActor)))))

(event OnComponentBeginOverlap(SwordCollision)
  (params (OverlappedComponent :type Primitive%20Component%20Object%20Reference) (OtherActor :type Actor%20Object%20Reference) (OtherComp :type Primitive%20Component%20Object%20Reference) (OtherBodyIndex :type Integer) (bFromSweep :type Boolean) (SweepResult :type Hit%20Result%20Structure%20%28by%20ref%29))
  (if (!= OtherActor self)
    (bind _asbp_base_character (Utilities|Casting|CastToBP_BaseCharacter OtherActor))
    (bind _returnvalue (Class|BaseCharacter|IsHostile _asbp_base_character self))
    (if _returnvalue
      (Ability|SendGameplayEventtoActor self "(TagName=\"skill.melee.dealDamage\")" (Utilities|Struct|MakeGameplayEventData "(TagName=\"\")" 0 OtherActor)))))

(event Custom|MeleeAttack
  (Abilities|TryActivateAbilitybyClass (Variables|Default|GetAbilitySystemComponent) "/Game/Blueprints/Characters/GameplayAbilities/Melee/GA_Melee.GA_Melee_C" true))

(event Custom|HealthRegen
  (Abilities|TryActivateAbilitybyClass (Variables|Default|GetAbilitySystemComponent) "/Game/Blueprints/Characters/GameplayAbilities/HealthRegen/GA_HealthRegen.GA_HealthRegen_C" true))

(event Custom|Dash
  (Abilities|TryActivateAbilitybyClass (Variables|Default|GetAbilitySystemComponent) "/Game/Blueprints/Characters/GameplayAbilities/Dash/GA_Dash.GA_Dash_C" true))

(event Custom|PushCharacter
  (params (ImpulseDirection :type Vector) (ImpulseStrength :type Float%20%28single-precision%29) (StunDuration :type Float%20%28single-precision%29))
  (bind _charactermovement (Variables|Character|GetCharacterMovement))
  (Variables|Default|SetOriginalGround%20Friction (Variables|/Script/Engine.CharacterMovementComponent|GetGroundFriction _charactermovement))
  (Variables|/Script/Engine.CharacterMovementComponent|SetGroundFriction _charactermovement 0.0)
  (Physics|AddImpulse (Variables|Character|GetCharacterMovement) (* ImpulseDirection ImpulseStrength) true)
  (if (> StunDuration 0.0)
    (Class|BaseCharacter|HitStun StunDuration))
  (Utilities|FlowControl|Delay 0.3)
  (Variables|/Script/Engine.CharacterMovementComponent|SetGroundFriction (Variables|Character|GetCharacterMovement) (Variables|Default|GetOriginalGround%20Friction)))

(event EventBeginPlay
  (Class|BaseCharacter|AquireAbility "/Game/Blueprints/Characters/GameplayAbilities/Melee/GA_Melee.GA_Melee_C")
  (Class|BaseCharacter|AquireAbility "/Game/Blueprints/Characters/GameplayAbilities/HealthRegen/GA_HealthRegen.GA_HealthRegen_C")
  (Class|BaseCharacter|AquireAbility "/Game/Blueprints/Characters/GameplayAbilities/Dash/GA_Dash.GA_Dash_C"))

(event Collision|EventActorBeginOverlap
  (params (OtherActor :type Actor%20Object%20Reference)))

(event EventTick
  (params (DeltaSeconds :type Float%20%28single-precision%29)))

(event EventDie
  (bind _returnvalue (Animation|PlayAnimMontage "/Game/Blueprints/Characters/Animation/AM_Shinbi_Die.AM_Shinbi_Die" 1.0 "None"))
  (Utilities|FlowControl|Delay _returnvalue)
  (Actor|DestroyActor))

(fn ConstructionScript)

(fn SetCollisiontoPawn
  (params (NewCollisionResponse :type ECollisionResponse%20Enum :default "ECR_Overlap"))
  (Collision|SetCollisionResponsetoChannel (Variables|Default|GetCapsuleComponent) "ECC_Pawn" NewCollisionResponse))