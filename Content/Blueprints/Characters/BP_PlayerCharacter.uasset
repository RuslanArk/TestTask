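; BP_PlayerCharacter is the player character Blueprint, which keeps the player's on-screen health and mana displays up to date.
; Health and mana change events cast the controller to BP_PlayerControllerBase and set the PrimaryUI glass ball widgets to the current-to-max ratio.
; BeginPlay, overlap and Tick are disabled stubs, and the construction script only calls its parent.
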(event EventBeginPlay
  (|CallParentFunction) ; This node is disabled and will not be called.\nDrag off pins to build functionality.
)

(event Collision|EventActorBeginOverlap
  (params (OtherActor :type Actor%20Object%20Reference))
  (|CallParentFunction OtherActor) ; This node is disabled and will not be called.\nDrag off pins to build functionality.
)

(event EventTick
  (params (DeltaSeconds :type Float%20%28single-precision%29))
  (|CallParentFunction DeltaSeconds) ; This node is disabled and will not be called.\nDrag off pins to build functionality.
)

(event EventOnHealthChanged
  (params (Health :type Float%20%28single-precision%29) (MaxHealth :type Float%20%28single-precision%29))
  (bind _asbp_player_controller_base (Utilities|Casting|CastToBP_PlayerControllerBase (Pawn|GetController)))
  (Default|SetPercentage (Variables|/Game/UI/Widgets/WB_PrimaryUI.WB_PrimaryUI_C|GetHealth_GlassBall (Variables|/Game/Blueprints/BP_PlayerControllerBase.BP_PlayerControllerBase_C|GetPrimaryUI _asbp_player_controller_base)) (/ Health MaxHealth)))

(event EventOnManaChanged
  (params (Mana :type Float%20%28single-precision%29) (MaxMana :type Float%20%28single-precision%29))
  (bind _asbp_player_controller_base (Utilities|Casting|CastToBP_PlayerControllerBase (Pawn|GetController)))
  (Default|SetPercentage (Variables|/Game/UI/Widgets/WB_PrimaryUI.WB_PrimaryUI_C|GetMana_GlassBall (Variables|/Game/Blueprints/BP_PlayerControllerBase.BP_PlayerControllerBase_C|GetPrimaryUI _asbp_player_controller_base)) (/ Mana MaxMana)))

(fn ConstructionScript
  (|CallParentFunction))